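; BP_DeamonArms is a gate-related actor that shows animated demon arms on demand, with a material-driven appearance effect.
; The skeletal mesh starts hidden; StartDeamonArms reveals it, plays its animation once and creates a dynamic material instance.
; A timeline drives the material's Appear parameter forward on start, and DisapearArms reverses it without re-hiding the mesh.
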(event `self.ReceiveBeginPlay`
  (`SceneComponent.SetHiddenInGame` (`self.SkeletalMesh`) true false))

(event `StartDeamonArms`
  (bind _skeletalmesh (`self.SkeletalMesh`))
  (`SceneComponent.SetHiddenInGame` (`self.SkeletalMesh`) false false)
  (`SkeletalMeshComponent.PlayAnimation` _skeletalmesh "/Game/Gates/Skeleton/SK_ArmsDeamon_Anim.SK_ArmsDeamon_Anim" false)
  (bind _returnvalue (`PrimitiveComponent.CreateDynamicMaterialInstance` (`self.SkeletalMesh`) 0 (`PrimitiveComponent.GetMaterial` _skeletalmesh 0) "None"))
  (set `self.DM_Arms` _returnvalue)
  (`|ExecutionSequence`
    (:`then_1`
      (`PrimitiveComponent.SetMaterial` (`self.SkeletalMesh`) 0 (`self.DM_Arms`))
      (bind (_direction _appear) (`Timeline|Timeline` :!via `PlayFromStart` :!label _label)
        (:`Update`
          (`MaterialInstanceDynamic.SetScalarParameterValue` (`self.DM_Arms`) "Appear" _appear))))))

(event `DisapearArms`
  (goto _label :!via `ReverseFromEnd`))

(fn `UserConstructionScript`)