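; BP_Chain builds a chain of mesh links along a spline in the construction script, with no runtime logic.
; Link spacing is the mesh's X bounding size plus an offset, and the spline length sets the link count.
; Each link is an instanced static mesh aimed at the next spacing point.
; A FlipFlop adds a roll offset to every other link to alternate their orientation.
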(fn `GetLocationAtIndex`
  (params (Index :type Integer))
  (returns (Location :type "Vector Structure"))
  (return (`SplineComponent.GetLocationAtDistanceAlongSpline` (`self.Spline`) (* Index (`self.Spacing`)) "Local")))

(fn `UserConstructionScript`
  (locals (NewLocalVar :type "Rotator Structure" :default (struct)))
  (bind _mesh (`self.Mesh`))
  (bind _rotationoffset_roll (`KismetMathLibrary.BreakRotator` (`self.RotationOffset`)))
  (bind _instancedstaticmesh (`self.InstancedStaticMesh`))
  (bind (_min _max) (break `Box` (`StaticMesh.GetBoundingBox` _mesh)))
  (`StaticMeshComponent.SetStaticMesh` _instancedstaticmesh _mesh)
  (`SceneComponent.SetRelativeScale3D` _instancedstaticmesh (`self.Scale`))
  (bind _output_get (set `self.Spacing` (+ (`self.Offset`) (.x (- _max _min)))))
  (bind _output_get_2 (set `self.NumberOfIndex` (`KismetMathLibrary.FFloor` (/ (`SplineComponent.GetSplineLength` (`self.Spline`)) _output_get))))
  (for _index (range (+ _output_get_2 1))
    (bind _output_get_3 (set `self.CurrentIndex` _index))
    (`/Engine/EditorBlueprintResources/StandardMacros.FlipFlop`
      (:`A`
        (bind _location (`self.GetLocationAtIndex` _output_get_3))
        (bind (_returnvalue_roll _returnvalue_pitch _returnvalue_yaw) (`KismetMathLibrary.BreakRotator` (`KismetMathLibrary.MakeRotFromX` (- (`self.GetLocationAtIndex` (+ _output_get_3 1)) _location))))
        (`InstancedStaticMeshComponent.AddInstance` (`self.InstancedStaticMesh`) (`KismetMathLibrary.MakeTransform` _location (`KismetMathLibrary.MakeRotator` _returnvalue_roll _returnvalue_pitch _returnvalue_yaw)) false))
      (:`B`
        (`InstancedStaticMeshComponent.AddInstance` (`self.InstancedStaticMesh`) (`KismetMathLibrary.MakeTransform` _location (`KismetMathLibrary.MakeRotator` (+ _returnvalue_roll _rotationoffset_roll) _returnvalue_pitch _returnvalue_yaw)) false)))))