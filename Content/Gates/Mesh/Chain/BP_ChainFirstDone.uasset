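; Builds a configurable physics chain in the construction script, with link count, spacing and roll twist set by variables.
; The first pass adds static mesh links from the Billboard's location, each offset along X and rolled from the previous one.
; The second pass joins neighbouring links with physics constraints at their own X spacing.
; Flags can switch off physics on the first and last links to pin either end.
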(event `self.ReceiveBeginPlay`)

(fn `UserConstructionScript`
  (locals (NewLocalVar :type "Rotator Structure" :default (struct)))
  (bind _lasttransform (`self.LastTransform`))
  (bind _lasttransformconstraint (`self.LastTransformConstraint`))
  (bind _chainslinks (`self.ChainsLinks`))
  (bind _chainnumber (`self.ChainNumber`))
  (bind _chainslinks_2 (`self.ChainsLinks`))
  (bind _currentindexconstraint (`self.CurrentIndexConstraint`))
  (bind _returnvalue (- _chainnumber 1))
  (`|ExecutionSequence`
    (:`then_0`
      (for _index (range _chainnumber)
        (if (== _index 0)
          (bind _output_get (set `self.FirstTransform` (`KismetMathLibrary.MakeTransform` (`SceneComponent.RelativeLocation` (`self.Billboard`)))))
          (bind _output_get_2 (set `self.LastTransform` _output_get))
          (bind _returnvalue_2 (`AddComponent|NODE_AddStaticMeshComponent-0` :`RelativeTransform` _output_get_2))
          (`KismetArrayLibrary.Array_AddUnique` (`self.ChainsLinks`) _returnvalue_2)
          (else
            (bind _output_get_3 (set `self.CurrentTransform` (`KismetMathLibrary.MakeTransform` (`KismetMathLibrary.MakeVector` (+ (.x (.location _lasttransform)) (`self.OffsetLocation`)) (.y (.location _lasttransform)) (.z (.location _lasttransform))) (`KismetMathLibrary.MakeRotator` (+ (.roll (.rotation _lasttransform)) (`self.OffsetRotation`)) (.pitch (.rotation _lasttransform)) (.yaw (.rotation _lasttransform))))))
            (bind _output_get_4 (set `self.LastTransform` _output_get_3))
            (bind _returnvalue_3 (`AddComponent|NODE_AddStaticMeshComponent-1` :`RelativeTransform` _output_get_4))
            (`KismetArrayLibrary.Array_AddUnique` (`self.ChainsLinks`) _returnvalue_3)))))
    (:`then_1`
      (for _index_2 (range (+ _returnvalue 1))
        (bind _output_get_5 (set `self.CurrentIndexConstraint` _index_2))
        (if (== _output_get_5 0)
          (if (not (`self.FirstChainPhysics?`))
            (`PrimitiveComponent.SetSimulatePhysics` (`|GetArrayItem` (`self.ChainsLinks`)) false))
          (bind _output_get_6 (set `self.FirstTransformConstraint` (`KismetMathLibrary.MakeTransform` (`KismetMathLibrary.MakeVector` (- (.x (.location (`self.FirstTransform`))) 50.0) (.y (.location (`self.FirstTransform`))) (.z (.location (`self.FirstTransform`)))))))
          (bind _output_get_7 (set `self.LastTransformConstraint` _output_get_6))
          (bind _returnvalue_4 (`AddComponent|NODE_AddPhysicsConstraintComponent-3` :`RelativeTransform` _output_get_7))
          (`PhysicsConstraintComponent.SetConstrainedComponents` _returnvalue_4 (`|GetArrayItem` _chainslinks) "None" (`|GetArrayItem` _chainslinks 1) "None")
          (elif (== _output_get_5 _returnvalue)
            (if (not (`self.LastChainPhysics?`))
              (`PrimitiveComponent.SetSimulatePhysics` (`|GetArrayItem` (`self.ChainsLinks`) (`self.CurrentIndexConstraint`)) false))
            (else
              (bind _output_get_8 (set `self.CurrentTransformConstrait` (`KismetMathLibrary.MakeTransform` (`KismetMathLibrary.MakeVector` (+ (.x (.location _lasttransformconstraint)) (`self.OffsetLocationConstraints`)) (.y (.location _lasttransformconstraint)) (.z (.location _lasttransformconstraint))) (`KismetMathLibrary.MakeRotator` (.roll (.rotation _lasttransformconstraint)) (.pitch (.rotation _lasttransformconstraint)) (.yaw (.rotation _lasttransformconstraint))))))
              (bind _output_get_9 (set `self.LastTransformConstraint` _output_get_8))
              (bind _returnvalue_5 (`AddComponent|NODE_AddPhysicsConstraintComponent-2` :`RelativeTransform` _output_get_9))
              (`PhysicsConstraintComponent.SetConstrainedComponents` _returnvalue_5 (`|GetArrayItem` _chainslinks_2 _currentindexconstraint) "None" (`|GetArrayItem` _chainslinks_2 (+ _currentindexconstraint 1)) "None"))))))))