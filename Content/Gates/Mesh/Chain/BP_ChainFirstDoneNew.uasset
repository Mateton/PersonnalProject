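; Procedural chain actor that builds a physics-constrained run of mesh links from FirstChain and LastChain endpoint components.
; The construction script derives spacing from their distance and ChainNumber, then adds intermediate static meshes, using a FlipFlop to alternate a 90-degree rotation.
; A second pass adds physics constraints at link midpoints and offset beyond both ends, pairing entries from the link array.
; BeginPlay only re-caches the endpoint locations.
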(event `self.ReceiveBeginPlay`
  (set `self.LastLocation` (`SceneComponent.RelativeLocation` (`self.LastChain`)))
  (set `self.FirstLocation` (`SceneComponent.RelativeLocation` (`self.FirstChain`))))

(fn `UserConstructionScript`
  (bind _chainnumber (`self.ChainNumber`))
  (bind _chainslinks (`self.ChainsLinks`))
  (bind _chainslinks_2 (`self.ChainsLinks`))
  (bind _currentindexconstraint (`self.CurrentIndexConstraint`))
  (bind _chainslinks_3 (`self.ChainsLinks`))
  (bind _currentindexconstraint_2 (`self.CurrentIndexConstraint`))
  (bind _returnvalue (+ (`self.ChainNumber`) 1))
  (bind _relativerotation (`SceneComponent.RelativeRotation` (`self.FirstChain`)))
  (bind _returnvalue_2 (* (* (+ (`self.FirstLocation`) (`self.Direction`)) (`self.Spacing`)) (+ (`self.CurrentIndex`) (0.0 0.0 0.0))))
  (set `self.LastLocation` (`SceneComponent.RelativeLocation` (`self.LastChain`)))
  (set `self.FirstLocation` (`SceneComponent.RelativeLocation` (`self.FirstChain`)))
  (set `self.Direction` (`KismetMathLibrary.Normal` (- (`self.LastLocation`) (`self.FirstLocation`))))
  (bind _output_get (set `self.TotalLength` (`KismetMathLibrary.VSize` (- (`self.LastLocation`) (`self.FirstLocation`)))))
  (set `self.Spacing` (/ _output_get (`self.ChainNumber`)))
  (`|ExecutionSequence`
    (:`then_0`
      (for _index (range (+ _chainnumber 1))
        (bind _output_get_2 (set `self.CurrentIndex` _index))
        (if (== _output_get_2 0)
          (`KismetArrayLibrary.Array_AddUnique` (`self.ChainsLinks`) (`self.FirstChain`))
          (elif (== _output_get_2 _chainnumber)
            (`KismetArrayLibrary.Array_AddUnique` (`self.ChainsLinks`) (`self.LastChain`))
            (else
              (`/Engine/EditorBlueprintResources/StandardMacros.FlipFlop`
                (:`A`
                  (bind _returnvalue_3 (`AddComponent|NODE_AddStaticMeshComponent-9` :`RelativeTransform` (`KismetMathLibrary.MakeTransform` _returnvalue_2 (`KismetMathLibrary.ComposeRotators` _relativerotation (struct :`Roll` 90.0)))))
                  (`KismetArrayLibrary.Array_AddUnique` (`self.ChainsLinks`) _returnvalue_3))
                (:`B`
                  (bind _returnvalue_4 (`AddComponent|NODE_AddStaticMeshComponent-6` :`RelativeTransform` (`KismetMathLibrary.MakeTransform` _returnvalue_2 _relativerotation)))
                  (`KismetArrayLibrary.Array_AddUnique` (`self.ChainsLinks`) _returnvalue_4))))))))
    (:`then_1`
      (for _index_2 (range (+ _returnvalue 1))
        (bind _output_get_3 (set `self.CurrentIndexConstraint` _index_2))
        (if (== _output_get_3 0)
          (bind _returnvalue_5 (`AddComponent|NODE_AddPhysicsConstraintComponent-11` :`RelativeTransform` (`KismetMathLibrary.MakeTransform` (- (`self.FirstLocation`) (50.0 0.0 0.0)))))
          (`PhysicsConstraintComponent.SetConstrainedComponents` _returnvalue_5 (`|GetArrayItem` (`self.ChainsLinks`)) "None" (`|GetArrayItem` (`self.ChainsLinks`) 1) "None")
          (elif (== _output_get_3 _returnvalue)
            (bind _returnvalue_6 (`AddComponent|NODE_AddPhysicsConstraintComponent-13` :`RelativeTransform` (`KismetMathLibrary.MakeTransform` (+ (`self.LastLocation`) (50.0 0.0 0.0)))))
            (`PhysicsConstraintComponent.SetConstrainedComponents` _returnvalue_6 (`|GetArrayItem` _chainslinks _returnvalue) "None" (`|GetArrayItem` _chainslinks (- _returnvalue 1)) "None")
            (else
              (bind _output_get_4 (set `self.ConstraintCurrentLocation` (/ (+ (`SceneComponent.RelativeLocation` (`|GetArrayItem` _chainslinks_2 _currentindexconstraint)) (`SceneComponent.RelativeLocation` (`|GetArrayItem` _chainslinks_2 (- _currentindexconstraint 1)))) 2.0)))
              (bind _returnvalue_7 (`AddComponent|NODE_AddPhysicsConstraintComponent-14` :`RelativeTransform` (`KismetMathLibrary.MakeTransform` _output_get_4)))
              (`PhysicsConstraintComponent.SetConstrainedComponents` _returnvalue_7 (`|GetArrayItem` _chainslinks_3 _currentindexconstraint_2) "None" (`|GetArrayItem` _chainslinks_3 (+ _currentindexconstraint_2 1)) "None"))))))))