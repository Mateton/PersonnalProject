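; Gate actor that plays a portal activation effect with flames, lights and glowing brick runes.
; ActivateFlame fires six flame effects and shows their point lights.
; Start triggers ActivateGate, then after a short delay activates Gate and raises the Bricks' emissive through a dynamic material instance.
; Reset hides the lights and destroys the flame and ActivateGate components rather than deactivating them, leaving Gate and runes untouched.
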(event `ActivateFlame`
  ; ActivateVFXFlame
  (`ActorComponent.Activate` (`self.Flame01`) false)
  (`ActorComponent.Activate` (`self.Flame06`) false)
  (`ActorComponent.Activate` (`self.Flame05`) false)
  (`ActorComponent.Activate` (`self.Flame04`) false)
  (`ActorComponent.Activate` (`self.Flame02`) false)
  (`ActorComponent.Activate` (`self.Flame03`) false)
  ; Light
  (`SceneComponent.SetVisibility` (`self.PointLight1`) true false)
  (`SceneComponent.SetVisibility` (`self.PointLight3`) true false)
  (`SceneComponent.SetVisibility` (`self.PointLight4`) true false)
  (`SceneComponent.SetVisibility` (`self.PointLight5`) true false)
  (`SceneComponent.SetVisibility` (`self.PointLight2`) true false)
  (`SceneComponent.SetVisibility` (`self.PointLight`) true false))

(event `Start`
  ; StartPortal
  (`ActorComponent.Activate` (`self.ActivateGate`) false)
  (`KismetSystemLibrary.Delay` 1.5)
  (`|ExecutionSequence`
    (:`then_0`
      ; AcitaveGate
      (`ActorComponent.Activate` (`self.Gate`) false))
    (:`then_1`
      ; ActivateRune
      (bind _returnvalue (`KismetMaterialLibrary.CreateDynamicMaterialInstance` (`PrimitiveComponent.GetMaterial` (`self.Bricks`) 0)))
      (bind _output_get (set `self.DM_BricksRunes` _returnvalue))
      (`PrimitiveComponent.SetMaterial` (`self.Bricks`) 0 _output_get)
      (`MaterialInstanceDynamic.SetScalarParameterValue` _output_get "Emissive" 5.0))))

(event `Reset`
  (`ActorComponent.K2_DestroyComponent` (`self.Flame03`))
  (`ActorComponent.K2_DestroyComponent` (`self.ActivateGate`))
  (`ActorComponent.K2_DestroyComponent` (`self.Flame06`))
  (`ActorComponent.K2_DestroyComponent` (`self.Flame05`))
  (`ActorComponent.K2_DestroyComponent` (`self.Flame03`))
  (`ActorComponent.K2_DestroyComponent` (`self.Flame01`))
  (`ActorComponent.K2_DestroyComponent` (`self.Flame02`))
  (`ActorComponent.K2_DestroyComponent` (`self.Flame04`))
  (`SceneComponent.SetVisibility` (`self.PointLight1`) false false)
  (`SceneComponent.SetVisibility` (`self.PointLight3`) false false)
  (`SceneComponent.SetVisibility` (`self.PointLight4`) false false)
  (`SceneComponent.SetVisibility` (`self.PointLight5`) false false)
  (`SceneComponent.SetVisibility` (`self.PointLight2`) false false)
  (`SceneComponent.SetVisibility` (`self.PointLight`) false false))

(fn `UserConstructionScript`)