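; BP_Dissolution is a Vampire effect actor that dissolves three skeletal meshes while particles are attracted toward a Caster component.
; Two seconds after BeginPlay, it passes the Caster's location to three Niagara systems as their attraction point, then activates them.
; A timeline then drives GetMaterial on each mesh, setting the Dissolution scalar on material slots 0 and 1 through dynamic material instances requested every update.
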(event `self.ReceiveBeginPlay`
  (`KismetSystemLibrary.Delay` 2.0)
  (`|ExecutionSequence`
    (:`then_0`
      ; Set AttractionPosition
      (bind _output_get (set `self.CasterLocation` (`SceneComponent.K2_GetComponentLocation` (`self.Caster`))))
      (`FXSystemComponent.SetVectorParameter` (`self.Niagara1`) "AttractionPointPosition" _output_get)
      (`FXSystemComponent.SetVectorParameter` (`self.Niagara`) "AttractionPointPosition" (`self.CasterLocation`))
      (`FXSystemComponent.SetVectorParameter` (`self.Niagara2`) "AttractionPointPosition" (`self.CasterLocation`)))
    (:`then_1`
      ; ActivateVFX
      (`ActorComponent.Activate` (`self.Niagara1`) false)
      (`ActorComponent.Activate` (`self.Niagara`) false)
      (`ActorComponent.Activate` (`self.Niagara2`) false))
    (:`then_2`
      (bind (_direction _newtrack_0) (`Timeline|Dissolution_Timeline` :!via `PlayFromStart`)
        (:`Update`
          (`self.GetMaterial` (`self.SkeletalMesh`) _newtrack_0)
          (`self.GetMaterial` (`self.SkeletalMesh1`) _newtrack_0)
          (`self.GetMaterial` (`self.SkeletalMesh2`) _newtrack_0))))))

(fn `GetMaterial`
  (params (SkeletalMesh :type "PrimitiveComponent Object Reference") (Dissolution :type "Float (double-precision)"))
  (locals (DM_02_Index :type "MaterialInstanceDynamic Object Reference") (DM_01_Index :type "MaterialInstanceDynamic Object Reference") (Target :type "PrimitiveComponent Object Reference") (Dissolutio :type "Float (double-precision)"))
  (bind _target (`local.Target`))
  (bind _dissolutio (`local.Dissolutio`))
  (set `local.Dissolutio` Dissolution)
  (bind _output_get (set `local.Target` SkeletalMesh))
  (`|ExecutionSequence`
    (:`then_0`
      (bind _returnvalue (`PrimitiveComponent.CreateDynamicMaterialInstance` _output_get 0 (`PrimitiveComponent.GetMaterial` _output_get 0) "None"))
      (bind _output_get_2 (set `local.DM_01_Index` _returnvalue))
      (`PrimitiveComponent.SetMaterial` _target 0 _output_get_2)
      (`MaterialInstanceDynamic.SetScalarParameterValue` _output_get_2 "Dissolution" _dissolutio))
    (:`then_1`
      (bind _returnvalue_2 (`PrimitiveComponent.CreateDynamicMaterialInstance` _output_get 1 (`PrimitiveComponent.GetMaterial` _output_get 1) "None"))
      (bind _output_get_3 (set `local.DM_02_Index` _returnvalue_2))
      (`PrimitiveComponent.SetMaterial` _target 1 _output_get_3)
      (`MaterialInstanceDynamic.SetScalarParameterValue` _output_get_3 "Dissolution" _dissolutio))))

(fn `UserConstructionScript`)